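; Wall-mounted air conditioner prop with a spinning fan, adjustable dirt and a fan sound.
; The construction script pushes the Dirt value into the fan and body materials, scales sound volume by fan RPM and a multiplier, and gives the fan a random starting angle.
; Tick rotates the fan around its pitch axis at a rate converted from FanRPM.
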(event EventBeginPlay)

(event Collision|EventActorBeginOverlap
  (params (OtherActor :type Actor%20Object%20Reference)))

(event EventTick
  (params (DeltaSeconds :type Float%20%28single-precision%29))
  (Transformation|AddLocalRotation (Variables|Default|GetFan) (Math|Rotator|MakeRotator 0.0 (* DeltaSeconds -6.0 (Variables|AirConditioner|GetFan%20RPM)) 0.0) false false))

(fn ConstructionScript
  (Rendering|Material|SetScalarParameterValueonMaterials (Variables|Default|GetFan) "Dirt" (Variables|AirConditioner|GetDirt))
  (Audio|Components|Audio|SetVolumeMultiplier (Variables|Default|GetSound) (* (Math|Float|Clamp(Float) (/ (- (Variables|AirConditioner|GetFan%20RPM) 6e+01) 1.9e+02)) (Variables|AirConditioner|GetVolume%20Multiplier)) :!class /Script/Engine.AudioComponent)
  (Transformation|AddLocalRotation (Variables|Default|GetFan) (Math|Rotator|MakeRotator 0.0 (Math|Random|RandomFloatinRange 0.0 3.6e+02) 0.0) false false) ; Random rotation for AC instance
)